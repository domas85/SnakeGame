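; BP_MenuGameMode is the menu's game mode, handling the transition from the menu into gameplay or out of the game.
; On BeginPlay it binds to the GameStateMachineSubsystem's game state change event.
; Entering Play saves data through PersistentGameDataSubsystem, hides the cursor, switches input to game-only and opens the gameplay level.
; Entering Quit exits the game.
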(event Custom|OnGameStateChanged
  (params (OldGameState :type EGameState%20Enum :default "Init") (NewGameState :type EGameState%20Enum :default "Init"))
  (bind _returnvalue (Game|GetPlayerController 0))
  (switch Utilities|FlowControl|Switch|SwitchonEGameState NewGameState
    (:Play
      (Class|PersistentGameDataSubsystem|SaveGameData (Subsystems|GetPersistentGameDataSubsystem))
      (Variables|/Script/Engine.PlayerController|SetbShowMouseCursor _returnvalue false)
      (Input|SetInputModeGameOnly _returnvalue false)
      (Game|OpenLevel(byObjectReference) "/Game/Maps/GamePlayLevel.GamePlayLevel"))
    (:Quit
      (Game|QuitGame 0 "Quit" false))))

(event EventBeginPlay
  (EventDispatchers|BindEventtoOnGameStateChanged (Subsystems|GetGameStateMachineSubsystem) (delegate Custom|OnGameStateChanged)))

(fn ConstructionScript)