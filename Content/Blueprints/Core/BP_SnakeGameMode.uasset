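; Game mode for the snake game that handles match startup, local multiplayer spawning and the switch to the game-over level.
; BeginPlay caches the SnakeGameState, loads persistent game data, creates extra local players from the saved count and links the second snake pawn to the first.
; Pawns teleport to PlayerStarts whose numeric tag equals their array index.
; A state-machine subsystem event opens the game-over level after a short delay.
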(event Custom|OnGameStateChanged
  (params (OldGameState :type EGameState%20Enum :default "Init") (NewGameState :type EGameState%20Enum :default "Init"))
  (switch Utilities|FlowControl|Switch|SwitchonEGameState NewGameState
    (:GameOver
      (Utilities|FlowControl|Delay 3.0)
      (Game|OpenLevel(byObjectReference) "/Game/Maps/GameOverLevel.GameOverLevel"))))

(event EventBeginPlay
  (EventDispatchers|BindEventtoOnGameStateChanged (Subsystems|GetGameStateMachineSubsystem) (EventDispatchers|CreateEvent :!event Custom|OnGameStateChanged))
  (CallFunction|Init)
  (for _index (range 2 (Class|PersistentGameDataSubsystem|GetNumPlayers (Subsystems|GetPersistentGameDataSubsystem)))
    (Class|GameplayStatics|CreatePlayer -1)
    (bind _asbp_snake_pawn (Utilities|Casting|CastToBP_SnakePawn (Game|Player|GetPlayerPawn 0)))
    (bind _asbp_snake_pawn_2 (Utilities|Casting|CastToBP_SnakePawn (Game|Player|GetPlayerPawn 1)))
    (Variables|/Game/Blueprints/Player/BP_SnakePawn.BP_SnakePawn_C|SetPlayer2 _asbp_snake_pawn _asbp_snake_pawn_2))
  (bind _outactors (Actor|GetAllActorsOfClass "/Script/Engine.PlayerStart"))
  (for (_array_element _array_index) _outactors
    (Utilities|IsValid _array_element
      (:Is%20Valid
        (if (== _array_index (Math|Conversions|ToInteger(Byte) (Utilities|String|ToString(Name) (Variables|/Script/Engine.PlayerStart|GetPlayerStartTag _array_element))))
          (Utilities|IsValid (Game|Player|GetPlayerPawn _array_index)
            (:Is%20Valid
              (Transformation|SetActorLocation (Game|Player|GetPlayerPawn _array_index) (Transformation|GetActorLocation _array_element) false true))))))))

(event EventPostLogin
  (params (NewPlayer :type Player%20Controller%20Object%20Reference))
  (Development|PrintString (Utilities|String|Append "Player logged in: " (Utilities|GetDisplayName NewPlayer)) true true "(R=0.000000,G=1.000000,B=0.000000,A=1.000000)" 2e+01))

(fn ConstructionScript)

(fn Init
  (bind _assnake_game_state (Utilities|Casting|CastToSnakeGameState (Game|GetGameState))
    (:then
      (Variables|Default|SetSnake%20Game%20State _assnake_game_state)
      (Class|PersistentGameDataSubsystem|LoadGameData (Subsystems|GetPersistentGameDataSubsystem))
      (Development|PrintString (Utilities|String|Append "Starting game with game type: " (Utilities|String|EnumtoString (Class|SnakeGameState|GetGameType (Variables|Default|GetSnake%20Game%20State))))))
    (:CastFailed
      (Development|PrintString "Failed get snake game state" true true "(R=1.000000,G=0.000000,B=0.000000,A=1.000000)" 8.0))))