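; Player snake pawn for a grid-based snake game, which also drives an optional second snake through its Player2 reference.
; On start it binds to BP_SnakeWorld's map changes, spawns apples by game type and reads human or AI player types.
; Enhanced Input steers both snakes, gated only by Player 1 being human, while AI snakes take A* directions at start or on F.
; Apple overlaps trigger eating, effects and an apple respawn.
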(event OnComponentBeginOverlap(CollisionComponent)
  (params (OverlappedComponent :type Primitive%20Component%20Object%20Reference) (OtherActor :type Actor%20Object%20Reference) (OtherComp :type Primitive%20Component%20Object%20Reference) (OtherBodyIndex :type Integer) (bFromSweep :type Boolean) (SweepResult :type Hit%20Result%20Structure%20%28by%20ref%29))
  (bind _asbp_apple (Utilities|Casting|CastToBP_Apple OtherActor))
  (Utilities|IsValid _asbp_apple
    (:Is%20Valid
      (Class|SnakePawn|AteApple)
      (Niagara|SpawnSystematLocation "/Game/Particles/NS_AppleVFX.NS_AppleVFX" (Transformation|GetActorLocation _asbp_apple))
      (Audio|SpawnSoundatLocation "/Game/Sounds/AppleAte.AppleAte" (Transformation|GetActorLocation _asbp_apple) "0, 0, 0" 1.0 (Math|Random|RandomFloatinRange 0.6 1.0) 0.0 0 0)
      (Class|SnakeWorld|SpawnApple (Variables|Default|GetGrid) _asbp_apple))))

(event Input|EnhancedActionEvents|EnhancedInputActionIA_MoveUp
  (params (ActionValue :type Boolean) (ElapsedSeconds :type Float%20%28double-precision%29) (TriggeredSeconds :type Float%20%28double-precision%29) (InputAction :type Input%20Action%20Object%20Reference :default "/Game/Input/Actions/IA_MoveUp.IA_MoveUp"))
  (if (Variables|Default|GetisPlayer1Human)
    (Class|SnakePawn|SetSnakeMoveDirrection "Up")))

(event Input|EnhancedActionEvents|EnhancedInputActionIA_MoveRight
  (params (ActionValue :type Boolean) (ElapsedSeconds :type Float%20%28double-precision%29) (TriggeredSeconds :type Float%20%28double-precision%29) (InputAction :type Input%20Action%20Object%20Reference :default "/Game/Input/Actions/IA_MoveRight.IA_MoveRight"))
  (if (Variables|Default|GetisPlayer1Human)
    (Class|SnakePawn|SetSnakeMoveDirrection "Right")))

(event Input|EnhancedActionEvents|EnhancedInputActionIA_MoveLeft
  (params (ActionValue :type Boolean) (ElapsedSeconds :type Float%20%28double-precision%29) (TriggeredSeconds :type Float%20%28double-precision%29) (InputAction :type Input%20Action%20Object%20Reference :default "/Game/Input/Actions/IA_MoveLeft.IA_MoveLeft"))
  (if (Variables|Default|GetisPlayer1Human)
    (Class|SnakePawn|SetSnakeMoveDirrection "Left")))

(event Input|EnhancedActionEvents|EnhancedInputActionIA_MoveDown
  (params (ActionValue :type Boolean) (ElapsedSeconds :type Float%20%28double-precision%29) (TriggeredSeconds :type Float%20%28double-precision%29) (InputAction :type Input%20Action%20Object%20Reference :default "/Game/Input/Actions/IA_MoveDown.IA_MoveDown"))
  (if (Variables|Default|GetisPlayer1Human)
    (Class|SnakePawn|SetSnakeMoveDirrection "Down")))

(event Input|EnhancedActionEvents|EnhancedInputActionIA_MoveUpP2
  (params (ActionValue :type Boolean) (ElapsedSeconds :type Float%20%28double-precision%29) (TriggeredSeconds :type Float%20%28double-precision%29) (InputAction :type Input%20Action%20Object%20Reference :default "/Game/Input/Actions/IA_MoveUpP2.IA_MoveUpP2"))
  (bind _player2 (Variables|Default|GetPlayer2))
  (if (Variables|Default|GetisPlayer1Human)
    (Utilities|IsValid _player2
      (:Is%20Valid
        (Class|SnakePawn|SetSnakeMoveDirrection _player2 "Up")))))

(event Input|EnhancedActionEvents|EnhancedInputActionIA_MoveDownP2
  (params (ActionValue :type Boolean) (ElapsedSeconds :type Float%20%28double-precision%29) (TriggeredSeconds :type Float%20%28double-precision%29) (InputAction :type Input%20Action%20Object%20Reference :default "/Game/Input/Actions/IA_MoveDownP2.IA_MoveDownP2"))
  (bind _player2 (Variables|Default|GetPlayer2))
  (if (Variables|Default|GetisPlayer1Human)
    (Utilities|IsValid _player2
      (:Is%20Valid
        (Class|SnakePawn|SetSnakeMoveDirrection _player2 "Down")))))

(event Input|EnhancedActionEvents|EnhancedInputActionIA_MoveRightP2
  (params (ActionValue :type Boolean) (ElapsedSeconds :type Float%20%28double-precision%29) (TriggeredSeconds :type Float%20%28double-precision%29) (InputAction :type Input%20Action%20Object%20Reference :default "/Game/Input/Actions/IA_MoveRightP2.IA_MoveRightP2"))
  (bind _player2 (Variables|Default|GetPlayer2))
  (if (Variables|Default|GetisPlayer1Human)
    (Utilities|IsValid _player2
      (:Is%20Valid
        (Class|SnakePawn|SetSnakeMoveDirrection _player2 "Right")))))

(event Input|EnhancedActionEvents|EnhancedInputActionIA_MoveLeftP2
  (params (ActionValue :type Boolean) (ElapsedSeconds :type Float%20%28double-precision%29) (TriggeredSeconds :type Float%20%28double-precision%29) (InputAction :type Input%20Action%20Object%20Reference :default "/Game/Input/Actions/IA_MoveLeftP2.IA_MoveLeftP2"))
  (bind _player2 (Variables|Default|GetPlayer2))
  (if (Variables|Default|GetisPlayer1Human)
    (Utilities|IsValid _player2
      (:Is%20Valid
        (Class|SnakePawn|SetSnakeMoveDirrection _player2 "Left")))))

(event EventBeginPlay
  (bind _player2 (Variables|Default|GetPlayer2))
  (CallFunction|Init)
  (Utilities|FlowControl|Sequence
    (:then_0
      (if (not (Variables|Default|GetisPlayer1Human))
        (bind _returnvalue (Class|SnakePawn|AStarDirection (Variables|Default|GetGrid)))
        (Class|SnakePawn|SetSnakeMoveDirrection _returnvalue)))
    (:then_1
      (Utilities|IsValid (Variables|Default|GetPlayer2)
        (:Is%20Valid
          (if (not (Variables|Default|GetisPlayer2Human))
            (bind _returnvalue_2 (Class|SnakePawn|AStarDirection _player2 (Variables|Default|GetGrid)))
            (Class|SnakePawn|SetSnakeMoveDirrection _player2 _returnvalue_2)))))))

(event EventTick
  (params (DeltaSeconds :type Float%20%28single-precision%29)))

(event Input|KeyboardEvents|F
  (params (Key :type Key%20Structure :default "None"))
  (bind _player2 (Variables|Default|GetPlayer2))
  (:Pressed
    (Utilities|FlowControl|Sequence
      (:then_0
        (if (not (Variables|Default|GetisPlayer1Human))
          (bind _returnvalue (Class|SnakePawn|AStarDirection (Variables|Default|GetGrid)))
          (Class|SnakePawn|SetSnakeMoveDirrection _returnvalue)))
      (:then_1
        (Utilities|IsValid (Variables|Default|GetPlayer2)
          (:Is%20Valid
            (if (not (Variables|Default|GetisPlayer2Human))
              (bind _returnvalue_2 (Class|SnakePawn|AStarDirection _player2 (Variables|Default|GetGrid)))
              (Class|SnakePawn|SetSnakeMoveDirrection _player2 _returnvalue_2))))))))

(fn ConstructionScript)

(fn DestroySnake
  (bind _childbodypart (Variables|Default|GetChildBodyPart))
  (Utilities|IsValid _childbodypart
    (:Is%20Valid
      (Class|SnakeBodyPart|KYS _childbodypart)
      (Actor|DestroyActor))
    (:Is%20Not%20Valid
      (Actor|DestroyActor))))

(fn RespawnSnake
  (bind _returnvalue (Game|SpawnActorfromClass "BP_SnakePawn_C" (Variables|Default|GetStartTransform) "Undefined" "MultiplyWithRoot" 0 (Game|GetInstigator (Game|GetPlayerController 0))))
  (Pawn|Possess (Game|GetPlayerController 0) _returnvalue))

(fn Init
  (bind _player2 (Variables|Default|GetPlayer2))
  (Variables|Default|SetStartTransform (Transformation|GetActorTransform))
  (bind _asplayer_controller (Utilities|Casting|CastToPlayerController (Pawn|GetController)))
  (Input|AddMappingContext (PlayerController|LocalPlayerSubsystems|GetEnhancedInputLocalPlayerSubsystem _asplayer_controller) "/Game/Input/IMC_PlayerSnake.IMC_PlayerSnake" 0 "(bIgnoreAllPressedKeysUntilRelease=True,bForceImmediately=False,bNotifyUserSettings=False)")
  (bind _returnvalue (Actor|GetActorOfClass "/Game/Blueprints/BP_SnakeWorld.BP_SnakeWorld_C"))
  (bind _output_get (Variables|Default|SetGrid _returnvalue))
  (EventDispatchers|BindEventtoMapChanged _output_get (EventDispatchers|CreateEvent :!event MoveSnaketoSpawn))
  (bind _asbp_snake_game_state (Utilities|Casting|CastToBP_SnakeGameState (Game|GetGameState)))
  (switch Utilities|FlowControl|Switch|SwitchonESnakeGameType (Class|SnakeGameState|GetGameType _asbp_snake_game_state)
    (:Cooperative
      (Class|SnakeWorld|SpawnApple (Variables|Default|GetGrid))
      (Class|SnakeWorld|SpawnApple (Variables|Default|GetGrid)))
    (:Battle
      (Class|SnakeWorld|SpawnApple (Variables|Default|GetGrid))))
  (for (_array_element _array_index) (Class|PersistentGameDataSubsystem|GetPlayersData (Subsystems|GetPersistentGameDataSubsystem))
    (CallFunction|SetIsHumanBool (.playertype _array_element) _array_index))
  ;[0.15 0.15 0.15 0.5] idk why the second player losses the grid reference
  (Utilities|IsValid _player2
    (:Is%20Valid
      (Variables|BP_SnakePawn_C|SetGrid _player2 (Variables|Default|GetGrid)))))

(fn MoveSnaketoSpawn
  (Class|SnakePawn|ClearMoveQueue)
  (Class|SnakePawn|SetSnakeMoveDirrection "Up")
  (Transformation|SetActorTransform (Variables|Default|GetStartTransform) false true))

(fn SetIsHumanBool
  (params (PlayerType :type EPlayerType%20Enum :default "None") (index :type Integer))
  (Utilities|FlowControl|Sequence
    (:then_0
      (if (== index 0)
        (switch Utilities|FlowControl|Switch|SwitchonEPlayerType PlayerType
          (:Human
            (Variables|Default|SetisPlayer1Human true))
          (:AI
            (Variables|Default|SetisPlayer1Human false)))))
    (:then_1
      (if (== index 1)
        (switch Utilities|FlowControl|Switch|SwitchonEPlayerType PlayerType
          (:Human
            (Variables|Default|SetisPlayer2Human true))
          (:AI
            (Variables|Default|SetisPlayer2Human false)))))))